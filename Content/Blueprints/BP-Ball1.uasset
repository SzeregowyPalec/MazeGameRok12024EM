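; BP-Ball1 is a player-controlled physics ball that rolls and jumps, fading in from black at level start.
; Both movement axes feed one torque node on the Sphere, while the jump axis applies an upward impulse gated by CanJump, which any hit re-arms.
; Any damage plays a death sound, fades to black and reloads the current level after a delay.
; An unconnected delayed-jump chain never runs.
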(event `self.ReceiveBeginPlay`
  (`PlayerCameraManager.StartCameraFade` :`self` (`GameplayStatics.GetPlayerCameraManager` 0) :`FromAlpha` 1.0 :`Duration` 4.0 :`bHoldWhenFinished` true))

(event `self.ReceiveAnyDamage`
  (params (Damage :type "Float (single-precision)") (DamageType :type "DamageType Object Reference") (InstigatedBy :type "Controller Object Reference") (DamageCauser :type "Actor Object Reference"))
  (`GameplayStatics.PlaySound2D` "/Game/StarterContent/Audio/Sekiro_Death_Sound_Effect.Sekiro_Death_Sound_Effect" 1.0 1.0 0.0 null null)
  (`PlayerCameraManager.StartCameraFade` :`self` (`GameplayStatics.GetPlayerCameraManager` 0) :`ToAlpha` 1.0 :`Duration` 4.0 :`bHoldWhenFinished` true)
  (`KismetSystemLibrary.Delay` 5.0)
  (bind _returnvalue (`GameplayStatics.GetCurrentLevelName` true))
  (`GameplayStatics.OpenLevel` (`KismetStringLibrary.Conv_StringToName` _returnvalue)))

(event `InputAxis|Moveback`
  (params (AxisValue :type "Float (single-precision)"))
  (bind _strmultiply (`self.StrMultiply`))
  (`PrimitiveComponent.AddTorqueInRadians` (`self.Sphere`) (`KismetMathLibrary.MakeVector` (* (stale `InputAxis|MoveLeftRight` AxisValue) _strmultiply) (* AxisValue _strmultiply)) "None" true :!label _label))

(event `Key|SpaceBar`
  (params (Key :type "Key Structure")))

(event `InputAxis|MoveLeftRight`
  (params (AxisValue :type "Float (single-precision)"))
  (goto _label))

(event `InputAxis|Movejump`
  (params (AxisValue :type "Float (single-precision)"))
  (if (`self.CanJump`)
    (`PrimitiveComponent.AddImpulse` (`self.Sphere`) (`KismetMathLibrary.MakeVector` 0.0 0.0 (* AxisValue (`self.Jumpheight`))) "None" true)
    (set `self.CanJump` false)))

(event `self.ReceiveHit`
  (params (MyComp :type "PrimitiveComponent Object Reference") (Other :type "Actor Object Reference") (OtherComp :type "PrimitiveComponent Object Reference") (bSelfMoved :type Boolean) (HitLocation :type "Vector Structure") (HitNormal :type "Vector Structure") (NormalImpulse :type "Vector Structure") (Hit :type "HitResult Structure (by ref)"))
  (set `self.CanJump` true))

(fn `UserConstructionScript`)
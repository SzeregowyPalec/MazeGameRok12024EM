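; A level-exit trigger volume that loads Level2 once no Crystal2 actors remain in the world.
; Any overlap with its box starts a camera fade-out, then after a delay the crystal check runs.
; Remaining crystals only trigger a Polish "not all crystals collected" debug print, and the fade is not reversed.
; Crystal1 actors are also gathered, but their check is disconnected, so only Crystal2 gates the exit.
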(event `self.Box.OnComponentBeginOverlap`
  (params (OverlappedComponent :type "PrimitiveComponent Object Reference") (OtherActor :type "Actor Object Reference") (OtherComp :type "PrimitiveComponent Object Reference") (OtherBodyIndex :type Integer) (bFromSweep :type Boolean) (SweepResult :type "HitResult Structure (by ref)"))
  (`PlayerCameraManager.StartCameraFade` :`self` (`GameplayStatics.GetPlayerCameraManager` 0) :`ToAlpha` 1.0 :`Duration` 4.0)
  (`KismetSystemLibrary.Delay` 3.0)
  (bind _outactors (`GameplayStatics.GetAllActorsOfClass` "/Game/Blueprints/Crystal1.Crystal1_C"))
  (bind _outactors_2 (`GameplayStatics.GetAllActorsOfClass` "/Game/Blueprints/Crystal2.Crystal2_C"))
  (if (> (`KismetArrayLibrary.Array_Length` _outactors_2) 0)
    (`KismetSystemLibrary.PrintString` "Nie zebrano wszytskich kryształów")
    (else
      (`GameplayStatics.OpenLevel` "Level2"))))

(fn `UserConstructionScript`)
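; Platform that tilts while the player's BP-Ball1 pawn is on it and levels out afterward.
; Box begin overlap sets the tilt flag by checking the actor against player pawn 0, while any end overlap clears it.
; Tick uses FInterpTo with slowed delta time to ease the Cube's roll toward the tilt angle or back to zero, holding pitch and yaw at zero.
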(event `self.Box.OnComponentBeginOverlap`
  (params (OverlappedComponent :type "PrimitiveComponent Object Reference") (OtherActor :type "Actor Object Reference") (OtherComp :type "PrimitiveComponent Object Reference") (OtherBodyIndex :type Integer) (bFromSweep :type Boolean) (SweepResult :type "HitResult Structure (by ref)"))
  (bind _asbp_ball_1 (cast `/Game/Blueprints/BP-Ball1` (`GameplayStatics.GetPlayerPawn` 0)))
  (if true
    (set `self.is Titing` (== _asbp_ball_1 OtherActor))))

(event `self.Box.OnComponentEndOverlap`
  (params (OverlappedComponent :type "PrimitiveComponent Object Reference") (OtherActor :type "Actor Object Reference") (OtherComp :type "PrimitiveComponent Object Reference") (OtherBodyIndex :type Integer))
  (set `self.is Titing` false))

(event `self.ReceiveTick`
  (params (DeltaSeconds :type "Float (single-precision)"))
  (bind _returnvalue (* DeltaSeconds 0.1))
  (bind _tilspeed (`self.Tilspeed`))
  (bind _cube (`self.Cube`))
  (bind _relativerotation_roll (`KismetMathLibrary.BreakRotator` (`SceneComponent.RelativeRotation` _cube)))
  (if (`self.is Titing`)
    (`SceneComponent.K2_SetRelativeRotation` _cube (`KismetMathLibrary.MakeRotator` (`KismetMathLibrary.FInterpTo` _relativerotation_roll (`self.Tiltangle`) _returnvalue _tilspeed)) false false)
    (else
      (`SceneComponent.K2_SetRelativeRotation` _cube (`KismetMathLibrary.MakeRotator` (`KismetMathLibrary.FInterpTo` _relativerotation_roll 0.0 _returnvalue _tilspeed)) false false))))

(fn `UserConstructionScript`)